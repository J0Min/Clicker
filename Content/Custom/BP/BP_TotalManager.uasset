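; Central manager for a clicker game, tracking currency, upgrade purchases and the HP of a destructible BP_StarBase.
; Clicks and a one-second timer add currency, pushed to WB_MainUI.
; SpawnUI buys DT_Upgrade entries by index, triggering drone, laser or stat upgrades, with costs scaling exponentially per purchase.
; UpdateProcessBar applies damage; at zero HP, Tick explodes the base once and shows the end screen.
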(event `/Game/Custom/BPI/BPI_Mange.IncreasePopUI`
  (params (Value :type Integer64))
  ; 클릭당 획득량 상승 보정 함수
  (bind _output_get (set `self.OneClickedAmount` (+ Value (`self.OneClickedAmount`))))
  (`KismetSystemLibrary.PrintString` (`KismetStringLibrary.Concat_StrStr` "현재 1클릭 획득량  " (`KismetStringLibrary.Conv_Int64ToString` _output_get))))

(event `SpawnActor`
  (params (Mesh :type "StaticMesh Object Reference"))
  ;[1 1 1] 액터 스폰
  (set `self.Array Element` Mesh)
  (for (_array_element _array_index) _
    (bind _ismached (`/Game/Custom/GoodBye/BP_SpawnArea.CompareMesh` _array_element Mesh))
    (if _ismached
      (bind (_out_row_upgrade_name _out_row_cost) (`self.MeshToName` (`self.Array Element`)))
      (bind _buy (`self.CompareAmount` _out_row_cost _array_index))
      (if _buy
        (`/Game/Custom/GoodBye/BP_SpawnArea.Spawn` _array_element)
        ; 액터 스폰 관련 상승량 보정
        (bind _outrownames (`DataTableFunctionLibrary.GetDataTableRowNames` "/Game/Custom/Data/DT_Upgrade.DT_Upgrade"))
        (for _array_element_2 _outrownames
          (bind _returnvalue (`|GetDataTableRow` "/Game/Custom/Data/DT_Upgrade.DT_Upgrade" _array_element_2)
            (:`then`
              (if (== (`.Actor_20_479C21164ADDEAEDC4FE6DB842B8698D` (break `/Game/Custom/Data/F_UpgradeData` _returnvalue)) (`self.Array Element`))
                (set `self.AutoClickAmount` (+ (`self.AutoClickAmount`) (`.Production_24_D79F8AE44CBE6EDA3F9BCC9376EB94B3` (break `/Game/Custom/Data/F_UpgradeData` _returnvalue))))))))
        (else
          (`KismetSystemLibrary.PrintString` "잔액 부족"))))))

(event `MulCost`
  (bind _buyamountdouble (`self.BuyAmountDouble`))
  ; cost 증가 반영 함수
  (bind _outrownames (`DataTableFunctionLibrary.GetDataTableRowNames` "/Game/Custom/Data/DT_Upgrade.DT_Upgrade"))
  (for (_array_element _array_index) _outrownames
    (bind _returnvalue (`|GetDataTableRow` "/Game/Custom/Data/DT_Upgrade.DT_Upgrade" _array_element)
      (:`then`
        (bind _output (`|GetArrayItem` (`self.NamesMatchBuyingAmount`) _array_index))
        (if (> _output 0)
          (bind _returnvalue_2 (* (`.Cost_12_38DB682D4A526BD222F3C486B22412F4` (break `/Game/Custom/Data/F_UpgradeData` _returnvalue)) (`KismetMathLibrary.MultiplyMultiply_FloatFloat` (`self.Multiplier`) (`KismetMathLibrary.Conv_IntToDouble` _output))))
          (`KismetArrayLibrary.Array_Set` _buyamountdouble _array_index _returnvalue_2)
          (`KismetSystemLibrary.PrintString` (`KismetStringLibrary.Conv_Int64ToString` _returnvalue_2))
          (`KismetSystemLibrary.PrintString` "구매")
          (`/Game/Custom/UI/WB_MainUI.InitList` (`self.mainUI`))
          (else
            (`KismetArrayLibrary.Array_Set` _buyamountdouble _array_index (`.Cost_12_38DB682D4A526BD222F3C486B22412F4` (break `/Game/Custom/Data/F_UpgradeData` _returnvalue)) true))))
      (:`RowNotFound`
        (`KismetSystemLibrary.PrintString` "잘못된 입력값")))))

(event `SpawnUI`
  (params (YourIndex :type Integer))
  (bind _namesmatchbuyingamount (`self.NamesMatchBuyingAmount`))
  (bind _your_index (`self.Your Index`))
  (set `self.Your Index` YourIndex)
  (bind _outrownames (`DataTableFunctionLibrary.GetDataTableRowNames` "/Game/Custom/Data/DT_Upgrade.DT_Upgrade"))
  (`|GetDataTableRow` "/Game/Custom/Data/DT_Upgrade.DT_Upgrade" (`|GetArrayItem` _outrownames (`self.Your Index`))
    (:`then`
      (if (> (`self.CurrentAmount`) (`|GetArrayItem` (`self.BuyAmountDouble`) (`self.Your Index`)))
        (`|ExecutionSequence`
          (:`then_0`
            (bind _result (`/Engine/EditorBlueprintResources/StandardMacros.IncrementInt` (`|GetArrayItem` _namesmatchbuyingamount _your_index))
              (:`  `
                (`KismetArrayLibrary.Array_Set` _namesmatchbuyingamount _your_index _result))))
          (:`then_1`
            (if (<= (`self.Your Index`) 1)
              (if (== (`self.Your Index`) 0)
                ; 1번 수습용 드론 스폰
                (`/Game/Custom/BP/BP_DroneManager.SpawnDrone` (`self.DroneManager`))
                (`self.MinusAmount`)
                (`self.MulCost`)
                (else
                  ; 2번 파괴용 레이저 스폰
                  (`/Game/Custom/BP/BP_StarBase.SpawnLaser` (`self.Base`))
                  (`self.MinusAmount`)
                  (`self.MulCost`)))
              (elif (== (`self.Your Index`) 2)
                ; 3번 데미지 증가
                (`/Engine/EditorBlueprintResources/StandardMacros.IncrementFloat` (`self.Damage`)
                  (:`  `
                    (`self.MinusAmount` :!label _label)
                    (`self.MulCost`)))
                (elif (== (`self.Your Index`) 3)
                  ; 4번 드론 속도 증가
                  (`/Game/Custom/BP/BP_DroneManager.IncresedDroneSpeed` (`self.DroneManager`))
                  (goto _label)
                  (else
                    (if (== (`self.Your Index`) 4)
                      ; 5번 파편량 증가
                      (bind _asbp_star_pawn (cast `/Game/Custom/BP/BP_StarPawn` (`GameplayStatics.GetPlayerPawn` 0)))
                      (`/Engine/EditorBlueprintResources/StandardMacros.IncrementInt` (`/Game/Custom/BP/BP_StarPawn.SpawnAmount` _asbp_star_pawn)
                        (:`  `
                          _))
                      (else
                        ; 6번 재화량 증가
                        (set `self.OneClickedAmount` (+ (`self.OneClickedAmount`) 1))))
                    (`self.MinusAmount`)
                    (`self.MulCost`)))))))
        (else
          (`KismetSystemLibrary.PrintString` "재화 부족" true true (struct :`R` 0.342043 :`G` 1.0 :`B` 0.164985 :`A` 1.0) 2.0 "Coin")
          (`/Game/Custom/UI/WB_MainUI.InitList` (`self.mainUI`)))))
    (:`RowNotFound`
      (`KismetSystemLibrary.PrintString` "잘못된 배열"))))

(event `VeryAmount`
  ; 재화량 증가(테스트함수)
  (set `self.CurrentAmount` 20000))

(event `/Game/Custom/BPI/BPI_Mange.AddCount`
  ; 1클릭
  (bind _output_get (set `self.CurrentAmount` (+ (`self.CurrentAmount`) (`self.OneClickedAmount`))))
  (set `/Game/Custom/UI/WB_MainUI.amount` _output_get (`self.mainUI`)))

(event `self.ReceiveBeginPlay`
  (`|ExecutionSequence`
    (:`then_0`
      ;[1 1 1] 메인 UI 생성
      (bind _returnvalue (`|CreateWidget` "/Game/Custom/UI/WB_MainUI.WB_MainUI_C" (`GameplayStatics.GetPlayerController` 0)))
      (bind _output_get (set `self.mainUI` _returnvalue))
      (`UserWidget.AddToViewport` _output_get 0)
      ; 게임 인스턴스 생성 및 할당
      (bind _asbp_game_instance (cast `/Game/Custom/BP/BP_GameInstance` (`GameplayStatics.GetGameInstance`)))
      (set `/Game/Custom/BP/BP_GameInstance.TotalManger` self _asbp_game_instance)
      ; base 추가
      (bind _returnvalue_2 (`GameplayStatics.GetActorOfClass` "/Game/Custom/BP/BP_StarBase.BP_StarBase_C"))
      (set `self.Base` _returnvalue_2)
      ; 코멘트
      (bind _returnvalue_3 (`GameplayStatics.GetActorOfClass` "/Game/Custom/BP/BP_DroneManager.BP_DroneManager_C"))
      (set `self.DroneManager` _returnvalue_3))
    (:`then_1`
      ; 메인 UI 변수들
      (bind _outrownames (`DataTableFunctionLibrary.GetDataTableRowNames` "/Game/Custom/Data/DT_Upgrade.DT_Upgrade"))
      (for _array_element _outrownames
        (bind _returnvalue_4 (`|GetDataTableRow` "/Game/Custom/Data/DT_Upgrade.DT_Upgrade" _array_element)
          (:`then`
            (`KismetArrayLibrary.Array_Add` (`self.Datatable Names`) (break `/Game/Custom/Data/F_UpgradeData` _returnvalue_4))
            (`KismetArrayLibrary.Array_Add` (`self.NamesMatchBuyingAmount`)))))
      (`/Game/Custom/UI/WB_MainUI.InitList` (`self.mainUI`)) ; 좌 상단 리스트 (스트링) 초기화
      (`self.MulCost`) ; 초기 코스트 초기화
    )
    (:`then_2`
      ; 코멘트
      (`KismetSystemLibrary.K2_SetTimerDelegate` (delegate `AutoClick`) 1.0 true)
      ; 최대 체력 처리 및 체력 바 업데이트
      (set `self.CurrentHP` (`self.MaxHP`))
      (`self.initialProcessBar`))))

(event `AutoClick`
  ; 자동 수확량 조정
  (bind _output_get (set `self.CurrentAmount` (+ (`self.CurrentAmount`) (`self.AutoClickAmount`))))
  (set `/Game/Custom/UI/WB_MainUI.amount` _output_get (`self.mainUI`)))

(event `UpdateProcessBar`
  (params (Damage :type "Float (double-precision)"))
  ; 체력깍기
  (bind _output_get (set `self.CurrentHP` (- (`self.CurrentHP`) Damage)))
  (bind _returnvalue (/ _output_get (`self.MaxHP`)))
  (`ProgressBar.SetPercent` (`/Game/Custom/UI/WB_MainUI.ProgressBar_0` (`self.mainUI`)) _returnvalue :!label _label_2)
  (`TextBlock.SetText` (`/Game/Custom/UI/WB_MainUI.BarText` (`self.mainUI`)) (`KismetTextLibrary.Conv_DoubleToText` (* _returnvalue 100.0) "HalfToEven" false true 1 324 3)))

(event `initialProcessBar`
  ; 체력깍기
  (goto _label_2))

(event `self.ReceiveTick`
  (params (DeltaSeconds :type "Float (single-precision)"))
  (bind _returnvalue_location (`KismetMathLibrary.BreakTransform` (`self.GetTransform` (`self.Base`))))
  (if (<= (* (/ (stale `UpdateProcessBar` _output_get) (`self.MaxHP`)) 100.0) 0.0)
    (`KismetSystemLibrary.PrintString` "BOMB")
    (`/Engine/EditorBlueprintResources/StandardMacros.DoOnce` false
      (:`Completed`
        (`NiagaraFunctionLibrary.SpawnSystemAtLocation` "/Game/MsvFx_Niagara_Explosion_Pack_01/Prefabs/Niagara_Dust_Explosion_01.Niagara_Dust_Explosion_01" _returnvalue_location (struct :`Pitch` 90.0))
        (`GameplayStatics.PlaySound2D` "/Game/Custom/TempFolder/explosion.explosion" 1.0 1.0 0.0 null null)
        (`self.K2_DestroyActor` (`self.Base`))
        (`KismetSystemLibrary.Delay` 2.0)
        (`self.EndLogic`)))))

(event `EndLogic`
  (bind _returnvalue (`GameplayStatics.GetPlayerController` 0))
  (set `PlayerController.bShowMouseCursor` true _returnvalue)
  (`WidgetBlueprintLibrary.SetInputMode_UIOnlyEx` _returnvalue null)
  (`Widget.RemoveFromParent` (`self.mainUI`))
  (bind _returnvalue_2 (`|CreateWidget` "/Game/Custom/UI/WB_End.WB_End_C" _returnvalue))
  (`UserWidget.AddToViewport` _returnvalue_2 0))

(fn `CompareAmount`
  (params (Price :type Integer64) (Index :type Integer))
  (returns (Buy :type Boolean))
  (locals (result :type Integer64)))

(fn `MeshToName`
  (params (NewParam :type "StaticMesh Object Reference"))
  (returns (`Out Row Upgrade Name` :type String) (`Out Row Cost` :type Integer64))
  (bind _outrownames (`DataTableFunctionLibrary.GetDataTableRowNames` "/Game/Custom/Data/DT_Upgrade.DT_Upgrade"))
  (for _array_element _outrownames
    (bind _returnvalue (`|GetDataTableRow` "/Game/Custom/Data/DT_Upgrade.DT_Upgrade" _array_element)
      (:`then`
        (if (== (`.Actor_20_479C21164ADDEAEDC4FE6DB842B8698D` (break `/Game/Custom/Data/F_UpgradeData` _returnvalue)) NewParam)
          (return (break `/Game/Custom/Data/F_UpgradeData` _returnvalue) (`.Cost_12_38DB682D4A526BD222F3C486B22412F4` (break `/Game/Custom/Data/F_UpgradeData` _returnvalue))))))))

(fn `MinusAmount`
  (set `self.CurrentAmount` (- (`self.CurrentAmount`) (`|GetArrayItem` (`self.BuyAmountDouble`) (`self.Your Index`)))))

(fn `UserConstructionScript`
  (`GameplayStatics.GetAllActorsOfClass` "/Game/Custom/GoodBye/BP_SpawnArea.BP_SpawnArea_C"))