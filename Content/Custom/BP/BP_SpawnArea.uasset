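; BP_SpawnArea is an actor that spawns BP_FirstPersonCharacter instances on a grid within its Box component on BeginPlay.
; Nested X and Y loops step by Spacing from the box's minimum corner, using counts derived from box size, and print a debug "Hello" per X step.
; The X loop takes the count as first index and 0 as last, the reverse of the Y loop.
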(event `self.ReceiveBeginPlay`
  (bind _spacing (`self.Spacing`))
  (bind _spacing_2 (`self.Spacing`))
  (bind (_origin _boxextent) (`KismetSystemLibrary.GetComponentBounds` (`self.Box`)))
  (for _index (range (`KismetMathLibrary.Conv_Int64ToInt` (`KismetMathLibrary.Conv_DoubleToInt64` (/ (.x (* _boxextent 2)) _spacing))) 1)
    (`KismetSystemLibrary.PrintString` "Hello")
    (for _index_2 (range (+ (`KismetMathLibrary.FTrunc` (/ (.y (* _boxextent 2)) _spacing)) 1))
      (`|SpawnActorFromClass` "/Game/FirstPerson/Blueprints/BP_FirstPersonCharacter.BP_FirstPersonCharacter_C" (`KismetMathLibrary.MakeTransform` (+ (- _origin _boxextent) (`KismetMathLibrary.MakeVector` (* _index _spacing_2) (* _index_2 _spacing_2)))) "Undefined" "MultiplyWithRoot" null null))))

(fn `UserConstructionScript`)