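; Player pawn that toggles an upgrade-slot menu and swings a pickaxe mesh.
; Tab drives a FlipFlop into Click, which creates or removes WBP_UpgradeSlot, switching cursor visibility and input mode.
; Left mouse press and release rotate the pickaxe by opposite relative offsets.
; BeginPlay caches a BP_Wooden actor, but its MovingHammerMessage call is disconnected and never runs.
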(event `Key|Tab` :paused true
  (params (Key :type "Key Structure"))
  (:`Pressed`
    (bind _isa (`/Engine/EditorBlueprintResources/StandardMacros.FlipFlop`)
      (:`A`
        _)
      (:`B`
        _))
    (bind _output_get (set `self.TapBool` _isa))
    (`self.Click`)))

(event `Click`
  (bind _returnvalue (`GameplayStatics.GetPlayerController` 0))
  (bind _returnvalue_2 (`GameplayStatics.GetPlayerController` 0))
  (if (stale `Key|Tab` _output_get)
    (bind _returnvalue_3 (`|CreateWidget` "/Game/Custom/UI/WBP_UpgradeSlot.WBP_UpgradeSlot_C"))
    (`UserWidget.AddToViewport` _returnvalue_3 0)
    (set `PlayerController.bShowMouseCursor` true _returnvalue)
    (`WidgetBlueprintLibrary.SetInputMode_GameAndUIEx` _returnvalue _returnvalue_3)
    (else
      (`Widget.RemoveFromParent` _returnvalue_3)
      (set `PlayerController.bShowMouseCursor` false _returnvalue_2)
      (`WidgetBlueprintLibrary.SetInputMode_GameOnly` _returnvalue_2))))

(event `self.ReceiveBeginPlay`
  (bind _returnvalue (`GameplayStatics.GetActorOfClass` "/Game/Custom/BP/BP_Wooden.BP_Wooden_C"))
  (set `self.Wood` _returnvalue))

(event `Key|LeftMouseButton`
  (params (Key :type "Key Structure"))
  (bind _sm_pickaxe (`self.SM_Pickaxe`))
  (:`Pressed`
    (`SceneComponent.K2_AddRelativeRotation` _sm_pickaxe (struct :`Roll` 90.0) false false))
  (:`Released`
    (`SceneComponent.K2_AddRelativeRotation` _sm_pickaxe (struct :`Roll` -90.0) false false)))

(fn `UserConstructionScript`)