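; Player pawn for a clicker-style mining game, swinging a pickaxe at a star.
; Left click tilts the pickaxe and sphere-traces from the camera; a StarBase hit spawns a radial burst of star dust and feeds damage to the GameInstance manager's progress bar.
; Tab toggles the upgrade widget with cursor and input mode, and key 1 toggles pause with a stop screen.
; Tick resets the clicks-per-second counter about every second.
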(event `Key|Tab` :paused true
  (params (Key :type "Key Structure"))
  (:`Pressed`
    (bind _isa (`/Engine/EditorBlueprintResources/StandardMacros.FlipFlop`)
      (:`A`
        _)
      (:`B`
        _))
    (bind _output_get (set `self.TapBool` _isa))
    (`self.Click`)))

(event `Click`
  (bind _returnvalue (`GameplayStatics.GetPlayerController` 0))
  (bind _returnvalue_2 (`GameplayStatics.GetPlayerController` 0))
  (if (stale `Key|Tab` _output_get)
    (bind _returnvalue_3 (`|CreateWidget` "/Game/Custom/UI/WBP_UpgradeSlot.WBP_UpgradeSlot_C"))
    (`UserWidget.AddToViewport` _returnvalue_3 0)
    (set `PlayerController.bShowMouseCursor` true _returnvalue)
    (`WidgetBlueprintLibrary.SetInputMode_GameAndUIEx` _returnvalue _returnvalue_3 "DoNotLock" false)
    (else
      (`Widget.RemoveFromParent` _returnvalue_3)
      (set `PlayerController.bShowMouseCursor` false _returnvalue_2)
      (`WidgetBlueprintLibrary.SetInputMode_GameOnly` _returnvalue_2)
      (`SceneComponent.K2_SetRelativeRotation` :`self` (`self.SM_Pickaxe`)))))

(event `Key|One` :paused true
  (params (Key :type "Key Structure"))
  (:`Pressed`
    (bind _isa (`/Engine/EditorBlueprintResources/StandardMacros.FlipFlop`)
      (:`A`
        (bind _returnvalue (`|CreateWidget` "/Game/Custom/UI/UI_Stop.UI_Stop_C"))
        (`UserWidget.AddToViewport` _returnvalue 0))
      (:`B`
        (`Widget.RemoveFromParent` _returnvalue)))
    (`GameplayStatics.SetGamePaused` _isa)))

(event `self.ReceiveBeginPlay`
  (bind _returnvalue (`GameplayStatics.GetActorOfClass` "/Game/Custom/BP/BP_StarBase.BP_StarBase_C"))
  (set `self.Star` _returnvalue))

(event `Key|LeftMouseButton`
  (params (Key :type "Key Structure"))
  (bind _cameracomponent (`self.CameraComponent`))
  (bind _sm_pickaxe (`self.SM_Pickaxe`))
  (bind _returnvalue (`SceneComponent.K2_GetComponentLocation` _cameracomponent))
  (:`Pressed`
    (`/Engine/EditorBlueprintResources/StandardMacros.IncrementInt` (`self.CPS`)
      (:`  `
        (`SceneComponent.K2_AddRelativeRotation` _sm_pickaxe (struct :`Roll` 90.0) false false)
        (bind _outhit (`KismetSystemLibrary.SphereTraceSingle` :`Start` _returnvalue :`End` (+ _returnvalue (* (`SceneComponent.GetForwardVector` _cameracomponent) (`self.Distance`))) :`Radius` 20.0 :`TraceChannel` "TraceTypeQuery1" :`DrawDebugType` "ForDuration"))
        (bind (_bblockinghit _binitialoverlap _time _distance _location _impactpoint _normal _impactnormal _physmat _hitactor) (`GameplayStatics.BreakHitResult` _outhit))
        (bind _asstar_base (cast `StarBase` _hitactor))
        (`StarBase.TriggerRadialSpawn` _asstar_base _location _normal "/Game/Custom/BP/BP_StarDust.BP_StarDust_C" (`self.SpawnAmount`) "/Game/Fab/Pack_Simple_Particle_Burst/01_Niagara_Systems/NS_Simple_Burst_Level_1.NS_Simple_Burst_Level_1" 200.0 70.0)
        (bind _asbp_game_instance (cast `/Game/Custom/BP/BP_GameInstance` (`GameplayStatics.GetGameInstance`)))
        (bind _totalmanger (`/Game/Custom/BP/BP_GameInstance.TotalManger` _asbp_game_instance))
        (`/Game/Custom/BP/BP_TotalManager.UpdateProcessBar` _totalmanger (`/Game/Custom/BP/BP_TotalManager.Damage` _totalmanger)))))
  (:`Released`
    (`SceneComponent.K2_AddRelativeRotation` _sm_pickaxe (struct :`Roll` -90.0) false false)))

(event `self.ReceiveTick`
  (params (DeltaSeconds :type "Float (single-precision)"))
  (bind _output_get (set `self.Second` (+ DeltaSeconds (`self.Second`))))
  (if (> _output_get 1.0)
    (set `self.CPS` 0)
    (set `self.Second` 0.0)))

(fn `UserConstructionScript`)