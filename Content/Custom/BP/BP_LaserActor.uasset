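; BP_LaserActor is a laser that periodically fires at StarBase actors to break star dust off them.
; A looping one-second timer runs a debug-drawn sphere trace forward from TargetArrow on the Visibility channel.
; On a StarBase hit, it triggers a radial spawn of a random few BP_StarDust actors with a Niagara burst at the impact point.
; It then passes Damage to the progress bar update on the GameInstance's TotalManger.
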(event `self.ReceiveBeginPlay`
  (`KismetSystemLibrary.K2_SetTimerDelegate` (delegate `QQQ`) 1.0 true))

(event `QQQ`
  (bind _targetarrow (`self.TargetArrow`))
  (bind _returnvalue (`SceneComponent.K2_GetComponentLocation` _targetarrow))
  (bind _outhit (`KismetSystemLibrary.SphereTraceSingle` :`Start` _returnvalue :`End` (+ _returnvalue (* (`SceneComponent.GetForwardVector` _targetarrow) 5000)) :`TraceChannel` "TraceTypeQuery1" :`DrawDebugType` "ForDuration"))
  (bind (_bblockinghit _binitialoverlap _time _distance _location _impactpoint _normal _impactnormal _physmat _hitactor) (`GameplayStatics.BreakHitResult` _outhit))
  (bind _asstar_base (cast `StarBase` _hitactor))
  (`StarBase.TriggerRadialSpawn` _asstar_base _location _normal "/Game/Custom/BP/BP_StarDust.BP_StarDust_C" (`KismetMathLibrary.RandomIntegerInRange` 1 5) "/Game/Fab/Pack_Simple_Particle_Burst/01_Niagara_Systems/NS_Simple_Burst_Level_1.NS_Simple_Burst_Level_1" 300.0 70.0)
  (bind _asbp_game_instance (cast `/Game/Custom/BP/BP_GameInstance` (`GameplayStatics.GetGameInstance`)))
  (`/Game/Custom/BP/BP_TotalManager.UpdateProcessBar` (`/Game/Custom/BP/BP_GameInstance.TotalManger` _asbp_game_instance) (`self.Damage`)))

(fn `UserConstructionScript`)