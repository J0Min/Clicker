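; BP_DroneManager spawns drones at its own transform, tracks them in an array, and sends them toward star dust.
; A looping timer searches for BP_StarDust actors, points each idle drone at one (in practice the first found) and marks it moving.
; When no dust remains it clears every drone's moving flag.
; A separate event raises the speed of all tracked drones.
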(event `IncresedDroneSpeed`
  ; 드론 속도 업
  (for _array_element (`self.Dron`)
    (set `/Game/Custom/BP/BP_Drone.Speed` (+ (`/Game/Custom/BP/BP_Drone.Speed` _array_element) (`self.IncreasedSpeedAmount`)) _array_element)))

(event `SpawnDrone`
  (bind _returnvalue (`|SpawnActorFromClass` "/Game/Custom/BP/BP_Drone.BP_Drone_C" (`self.GetTransform`) "AdjustIfPossibleButAlwaysSpawn" "MultiplyWithRoot" null false null))
  (`KismetArrayLibrary.Array_Add` (`self.Dron`) _returnvalue))

(event `self.ReceiveBeginPlay`
  (`KismetSystemLibrary.K2_SetTimerDelegate` (delegate `FindDust`) 0.5 true true))

(event `FindDust`
  (bind _outactors (`GameplayStatics.GetAllActorsOfClass` "/Game/Custom/BP/BP_StarDust.BP_StarDust_C"))
  (if (`KismetArrayLibrary.Array_IsEmpty` _outactors)
    (for _array_element (`self.Dron`)
      (set `/Game/Custom/BP/BP_Drone.isMoving` false _array_element))
    (else
      (for _array_element_2 _outactors
        (for _array_element_3 (`self.Dron`)
          (if (not (`/Game/Custom/BP/BP_Drone.isMoving` _array_element_3))
            (bind _returnvalue (`SceneComponent.K2_GetComponentLocation` (`/Game/Custom/BP/BP_Drone.SM_Drone` _array_element_3)))
            (bind _returnvalue_2 (`SceneComponent.K2_GetComponentLocation` (`/Game/Custom/BP/BP_StarDust.StaticMesh` _array_element_2)))
            (set `/Game/Custom/BP/BP_Drone.ToLocation` (`KismetMathLibrary.GetDirectionUnitVector` _returnvalue _returnvalue_2) _array_element_3)
            (set `/Game/Custom/BP/BP_Drone.isMoving` true _array_element_3)
            (`SceneComponent.K2_SetWorldRotation` (`/Game/Custom/BP/BP_Drone.Sphere` _array_element_3) (`KismetMathLibrary.FindLookAtRotation` _returnvalue _returnvalue_2) false false)))
        (`KismetSystemLibrary.PrintString` "다 일하고 있어요" true true (struct :`G` 0.66 :`B` 1.0 :`A` 1.0) 2.0 "1")))))

(fn `UserConstructionScript`)