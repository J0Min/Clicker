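; BP_Wooden is an actor with a hammer mesh that animates each time its QFunction event is called.
; QFunction prints a counter, increments it, then plays the Ham timeline from the start to drive the world pitch of SMHammer, passing in its relative roll and yaw.
; The Box overlap only casts to BP_FirstPersonCharacter, with no action after it.
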(event `self.ReceiveBeginPlay`)

(event `/Game/Custom/NewInterface.QFunction`
  (bind _count (`self.count`))
  (bind _sm_hammer (`self.SM_Hammer`))
  (bind (_relativerotation_roll _relativerotation_pitch _relativerotation_yaw) (`KismetMathLibrary.BreakRotator` (`SceneComponent.RelativeRotation` _sm_hammer)))
  (`KismetSystemLibrary.PrintString` (`KismetStringLibrary.Conv_IntToString` _count))
  (`/Engine/EditorBlueprintResources/StandardMacros.IncrementInt` _count
    (:`  `
      (bind (_direction `_새_트랙_0`) (`Timeline|Ham` :!via `PlayFromStart`)
        (:`Update`
          (`SceneComponent.K2_SetWorldRotation` _sm_hammer (`KismetMathLibrary.MakeRotator` _relativerotation_roll `_새_트랙_0` _relativerotation_yaw) false false))))))

(event `self.Box.OnComponentBeginOverlap`
  (params (OverlappedComponent :type "PrimitiveComponent Object Reference") (OtherActor :type "Actor Object Reference") (OtherComp :type "PrimitiveComponent Object Reference") (OtherBodyIndex :type Integer) (bFromSweep :type Boolean) (SweepResult :type "HitResult Structure (by ref)"))
  (cast `/Game/FirstPerson/Blueprints/BP_FirstPersonCharacter` OtherActor))

(fn `UserConstructionScript`)