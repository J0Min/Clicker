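; BP_SpawnArea is a spawn area Blueprint that stores a mesh and spawns actors with it.
; SetMesh assigns the stored mesh, and Spawn increments a call-frequency counter before passing that mesh to SpawnNextActorWithMesh, whose implementation is outside this graph.
; CompareMesh reports whether a given mesh matches the stored one.
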(event `Spawn`
  (`/Engine/EditorBlueprintResources/StandardMacros.IncrementInt` (`self.Callfrequency`)
    (:`  `
      (`self.SpawnNextActorWithMesh` (`self.Static`)))))

(event `SetMesh`
  (params (Mesh :type "StaticMesh Object Reference"))
  (set `self.Static` Mesh))

(fn `CompareMesh`
  (params (Mesh :type "Object Object Reference"))
  (returns (isMached :type Boolean))
  (if (== Mesh (`self.Static`))
    (return true)
    (else
      (return false))))

(fn `UserConstructionScript`)