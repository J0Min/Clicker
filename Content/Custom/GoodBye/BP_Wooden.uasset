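; BP_Wooden is a hammer-and-slime prop that animates a strike when MovingHammer is called.
; Each strike tells Manager to add a count message and spawns a BP_POP popup at the actor's transform.
; Two timelines play together: one pitches the hammer, the other drives the slime's Z scale, keeping the X and Y cached at BeginPlay.
; NewVar is false during the swing and true afterward; the Chop sound is disconnected.
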(event `/Game/Custom/BPI/BPI_HammerHit.MovingHammer`
  (bind (_slimescale_x _slimescale_y) (`KismetMathLibrary.BreakVector` (`self.SlimeScale`)))
  ; 매개체 내려칠때 팝업 UI생성
  (set `self.NewVar` false)
  (message `/Game/Custom/BPI/BPI_Mange.AddCount` (`self.Manager`))
  (`|SpawnActorFromClass` "/Game/Custom/GoodBye/BP_POP.BP_POP_C" (`self.GetTransform`) "Undefined" "MultiplyWithRoot" null null)
  (`|ExecutionSequence`
    (:`then_0`
      ; 망치 까딱
      (bind (_direction `_새_트랙_0`) (`Timeline|Ham` :!via `PlayFromStart`)
        (:`Update`
          (`SceneComponent.K2_SetWorldRotation` (`self.SM_Hammer`) (`KismetMathLibrary.MakeRotator` 0.0 `_새_트랙_0`) false false))
        (:`Finished`
          (set `self.NewVar` true))))
    (:`then_1`
      ; 슬라임 scale 조절
      (bind (_direction_2 `_새_트랙_0_2`) (`Timeline|타임라인` :!via `PlayFromStart`)
        (:`Update`
          (`SceneComponent.SetWorldScale3D` (`self.SM_Slim`) (`KismetMathLibrary.MakeVector` _slimescale_x _slimescale_y `_새_트랙_0_2`)))))))

(event `self.ReceiveBeginPlay`
  ; 중간 매개체 기본 스케일 저장
  (set `self.SlimeScale` (`SceneComponent.K2_GetComponentScale` (`self.SM_Slim`))))

(fn `UserConstructionScript`)